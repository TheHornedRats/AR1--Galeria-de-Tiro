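; BP_Target is a moving shootable target that changes the score when hit by a first-person projectile.
; Tick moves it along MoveDirection at MoveSpeed using a swept local offset.
; A projectile hit calls OnShot and destroys the projectile.
; OnShot sends PointValue, or HitPenalty when PointValue is not positive, to the first GameManager found, prints PointValue in green or red, then destroys the target.
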(event `self.ReceiveHit`
  (params (MyComp :type "PrimitiveComponent Object Reference") (Other :type "Actor Object Reference") (OtherComp :type "PrimitiveComponent Object Reference") (bSelfMoved :type Boolean) (HitLocation :type "Vector Structure") (HitNormal :type "Vector Structure") (NormalImpulse :type "Vector Structure") (Hit :type "HitResult Structure (by ref)"))
  (bind _asbp_first_person_projectile (cast `/Game/FirstPerson/Blueprints/BP_FirstPersonProjectile` Other))
  (`self.OnShot`)
  (`self.K2_DestroyActor` _asbp_first_person_projectile))

(event `OnShot`
  (bind _outactors (`GameplayStatics.GetAllActorsOfClass` "/Game/Corregir/Manager/GameManager.GameManager_C"))
  (if (> (`self.PointValue`) 0)
    (bind _output (`|GetArrayItem` _outactors))
    (`/Game/Corregir/Manager/GameManager.AddScore` _output (`self.PointValue`))
    (`KismetSystemLibrary.PrintString` (`KismetStringLibrary.Concat_StrStr` "+ " (`KismetStringLibrary.Conv_Int64ToString` (`self.PointValue`))) true true (struct :`R` 0.014317 :`G` 1.0 :`B` 0.10529 :`A` 1.0))
    (`self.K2_DestroyActor`)
    (else
      (`/Game/Corregir/Manager/GameManager.AddScore` _output (`self.HitPenalty`))
      (`KismetSystemLibrary.PrintString` (`KismetStringLibrary.Concat_StrStr` "- " (`KismetStringLibrary.Conv_Int64ToString` (`self.PointValue`))) true true (struct :`R` 1.0 :`B` 0.025802 :`A` 1.0))
      (`self.K2_DestroyActor`))))

(event `self.ReceiveTick`
  (params (DeltaSeconds :type "Float (single-precision)"))
  (`self.K2_AddActorLocalOffset` (* DeltaSeconds (`self.MoveDirection`) (`self.MoveSpeed`)) true))

(fn `UserConstructionScript`)