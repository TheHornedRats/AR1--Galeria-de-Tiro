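; BP_Spawner is a spawner that periodically creates target actors at its own transform.
; StartSpawning enables spawning and starts a looping timer that calls the SpawnTarget event.
; Each spawned BP_Target receives the default hit penalty, and a random roll against SpawnNegativeChance decides whether its point value is zero or the default.
; StopSpawning is an empty stub, so nothing here halts the timer.
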(event `SpawnTarget`
  (if (`self.bCanSpawn`)
    (bind _returnvalue (`|SpawnActorFromClass` (`self.TargetClass`) (`self.GetTransform`) "Undefined" "MultiplyWithRoot" null null))
    (bind _asbp_target (cast `/Game/Corregir/Targets/BP_Target` _returnvalue))
    (if (<= (`KismetMathLibrary.RandomFloatInRange` 0.0 1.0) (`self.SpawnNegativeChance`))
      (set `/Game/Corregir/Targets/BP_Target.PointValue` 0 _asbp_target)
      (set `/Game/Corregir/Targets/BP_Target.HitPenalty` (`self.HitPenalty-Default`) _asbp_target)
      (else
        (set `/Game/Corregir/Targets/BP_Target.PointValue` (`self.PointValue-Default`) _asbp_target)
        (set `/Game/Corregir/Targets/BP_Target.HitPenalty` (`self.HitPenalty-Default`) _asbp_target)))))

(fn `StartSpawning`
  (set `self.bCanSpawn` true)
  (`KismetSystemLibrary.K2_SetTimer` null "SpawnTarget" (`self.SpawnInterval`) true))

(fn `StopSpawning`)

(fn `UserConstructionScript`)